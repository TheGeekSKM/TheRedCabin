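; BP_WhiteBloodCell is an AI pawn that emerges from hiding and moves toward the player.
; On BeginPlay it drops its Sphere component by a fixed offset and records that height as the hidden position.
; ComeOut plays a timeline that lerps the Sphere back up at the actor's XY.
; When the rise finishes, it issues AIMoveTo on the player pawn and starts SCWhiteBloodCell playback at a random time.
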(event Custom|ComeOut
  (bind _returnvalue (Transformation|GetActorLocation))
  (bind _cellrise (Timeline|Timeline Play)
    (:Update
      (Transformation|SetWorldLocation (Variables|Default|GetSphere) (Math|Vector|MakeVector (.x _returnvalue) (.y _returnvalue) (Math|Float|Lerp (stale EventBeginPlay _output_get) (+ (stale EventBeginPlay _output_get) (Math|Float|MakeLiteralFloat 1.5e+02)) _cellrise)) false false))
    (:Finished
      (Utilities|FlowControl|Sequence
        (:then_0
          (AI|AIMoveTo self "0, 0, 0" (Game|Player|GetPlayerPawn 0) 5.0 false))
        (:then_1
          (Audio|Components|Audio|Play (Variables|Default|GetSC_WhiteBloodCell) (Math|Random|RandomFloatinRange 0.0 1e+01)))))))

(event EventBeginPlay
  (bind _sphere (Variables|Default|GetSphere))
  (Transformation|AddLocalOffset _sphere (Math|Vector|MakeVector 0.0 0.0 (* (Math|Float|MakeLiteralFloat 1.5e+02) -1.0)) false false)
  (bind _output_get (Variables|Default|SetHiddenHeight (.z (Transformation|GetWorldLocation _sphere)))))

(event Collision|EventActorBeginOverlap
  (params (OtherActor :type Actor%20Object%20Reference)))

(event EventTick
  (params (DeltaSeconds :type Float%20%28single-precision%29)))

(fn ConstructionScript)