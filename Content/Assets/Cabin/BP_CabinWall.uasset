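; Cabin wall Blueprint that procedurally builds a row of evenly spaced wooden logs from cylinder meshes with a triplanar plank material.
; All work happens in the Construction Script; the event graph is unused.
; WallType selects solid logs, an opening bounded by top and bottom indices, or one running from the first log to the top index.
; Logs within an opening split into left and right pieces, extending inward from both segment ends.
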(event EventBeginPlay)

(event Collision|EventActorBeginOverlap
  (params (OtherActor :type Actor%20Object%20Reference)))

(event EventTick
  (params (DeltaSeconds :type Float%20%28single-precision%29)))

(fn ConstructionScript
  (bind _walltype (Variables|Default|GetWallType))
  (bind _returnvalue (Utilities|Enum|Equal(Enum) _walltype "NewEnumerator1"))
  (bind _returnvalue_2 (Utilities|Enum|Equal(Enum) _walltype "NewEnumerator2"))
  (for _index (range 0 20)
    (LocalVariables|SetOffset (* (Math|Conversions|ToFloat(Integer) _index) -15.0))
    (LocalVariables|SetGap (and (and (<= _index (Variables|Default|GetGapTopHeight)) (or _returnvalue _returnvalue_2)) (or (and (>= _index (Variables|Default|GetGapBottomHeight)) _returnvalue) _returnvalue_2)))
    (Utilities|FlowControl|Sequence
      (:then_0
        (bind _returnvalue_3 (AddComponent|AddStaticMeshComponent false (Math|Transform|MakeTransform "0, 0, 0" "0.000000,0.000000,90.000000" (Math|Vector|MakeVector 0.2 0.2 (select (LocalVariables|GetGap) (Variables|Default|GetGapLeftSide) (Variables|Default|GetSegmentLength))))))
        (Components|StaticMesh|SetStaticMesh _returnvalue_3 "/Game/Assets/Cabin/SM_Cylinder.SM_Cylinder")
        (Rendering|Material|SetMaterial _returnvalue_3 0 "/Game/Assets/M_WoodPlanksTriplanar.M_WoodPlanksTriplanar")
        (Transformation|AddLocalOffset _returnvalue_3 (Math|Vector|MakeVector 0.0 (LocalVariables|GetOffset) 0.0) false false))
      (:then_1
        (if (LocalVariables|GetGap)
          (bind _returnvalue_4 (AddComponent|AddStaticMeshComponent false (Math|Transform|MakeTransform (Math|Vector|MakeVector 0.0 (* (Variables|Default|GetSegmentLength) 1e+02) 0.0) "180.000000,0.000000,-90.000000" (Math|Vector|MakeVector 0.2 0.2 (Variables|Default|GetGapRightSide)))))
          (Components|StaticMesh|SetStaticMesh _returnvalue_4 "/Game/Assets/Cabin/SM_Cylinder.SM_Cylinder")
          (Rendering|Material|SetMaterial _returnvalue_4 0 "/Game/Assets/M_WoodPlanksTriplanar.M_WoodPlanksTriplanar")
          (Transformation|AddLocalOffset _returnvalue_4 (Math|Vector|MakeVector 0.0 (LocalVariables|GetOffset) 0.0) false false))))))