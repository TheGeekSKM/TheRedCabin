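; Controller that drives a post-process material from the time of day of a referenced UDS actor.
; The construction script creates a dynamic instance of PPMI_PostProcess, adds it to a Post Process Volume as a blendable and sets its initial NormalizedTime.
; BeginPlay turns on outlines, and Tick converts the UDS time code into a 0–1 day fraction for NormalizedTime.
; Sun-light-driven fog color logic is present but never runs.
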(event EventBeginPlay
  (Rendering|Material|SetScalarParameterValue (Variables|Default|GetDynamicPPMaterial) "UseOutlines" 1.0 :!class /Script/Engine.MaterialInstanceDynamic))

(event Collision|EventActorBeginOverlap
  (params (OtherActor :type Actor%20Object%20Reference)))

(event EventTick
  (params (DeltaSeconds :type Float%20%28single-precision%29))
  (bind _uds_actor (Variables|Default|GetUDS%20Actor))
  (bind _time (Default|GetTimeCode _uds_actor))
  (Rendering|Material|SetScalarParameterValue (Variables|Default|GetDynamicPPMaterial) "NormalizedTime" (Math|Float|MapRangeUnclamped (Math|Conversions|ToFloat(Integer) (+ (+ (* (.hours _time) 3600) (* (.minutes _time) 60)) (.seconds _time))) 0.0 8.64e+04 0.0 1.0) :!class /Script/Engine.MaterialInstanceDynamic))

(fn ConstructionScript
  (bind _uds_actor (Variables|Default|GetUDS%20Actor))
  (bind _time (Default|GetTimeCode _uds_actor))
  (bind _returnvalue (Rendering|Material|CreateDynamicMaterialInstance "/Game/_Chris/PPMI_PostProcess.PPMI_PostProcess" "None" "None" :!class /Script/Engine.KismetMaterialLibrary))
  (bind _output_get (Variables|Default|SetDynamicPPMaterial _returnvalue))
  (Rendering|AddorUpdateBlendable (Variables|Default|GetPostProcessVolume) _output_get 1.0 :!class /Script/Engine.PostProcessVolume)
  (Rendering|Material|SetScalarParameterValue (Variables|Default|GetDynamicPPMaterial) "NormalizedTime" (Math|Float|MapRangeUnclamped (Math|Conversions|ToFloat(Integer) (+ (+ (* (.hours _time) 3600) (* (.minutes _time) 60)) (.seconds _time))) 0.0 8.64e+04 0.0 1.0) :!class /Script/Engine.MaterialInstanceDynamic))