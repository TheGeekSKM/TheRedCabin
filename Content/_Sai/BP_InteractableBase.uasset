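; Base actor for clickable world interactables that show a hover prompt to the first-person player.
; Construction applies the configured mesh and material to its static mesh component.
; On BeginPlay it caches the BP_FirstPersonCharacter and binds cursor-over events, showing or hiding that character's interaction widget with the name and left/right click hints.
; OnLeftClick and OnRightClick forward to empty LeftClick and RightClick events, presumably overridden by children.
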(event Custom|OnCursorOver
  (params (TouchedActor :type Actor%20Object%20Reference))
  (Default|ShowHover (Variables|/Game/FirstPerson/Blueprints/BP_FirstPersonCharacter.BP_FirstPersonCharacter_C|GetInteractionWidget (Variables|Default|GetPlayerPawn)) (Variables|Interactable|GetInteractableName) (Variables|Interactable|GetLeftClickInfo) (Variables|Interactable|GetRightClickInfo)))

(event Custom|OnCursorEnd
  (params (TouchedActor :type Actor%20Object%20Reference))
  (Default|HideHover (Variables|/Game/FirstPerson/Blueprints/BP_FirstPersonCharacter.BP_FirstPersonCharacter_C|GetInteractionWidget (Variables|Default|GetPlayerPawn))))

(event Custom|LeftClick
  (params (Player :type BP%20First%20Person%20Character%20Object%20Reference)))

(event Custom|RightClick
  (params (Player :type BP%20First%20Person%20Character%20Object%20Reference)))

(event EventBeginPlay
  (bind _asbp_first_person_character (Utilities|Casting|CastToBP_FirstPersonCharacter (Game|GetPlayerCharacter 0)))
  (Variables|Default|SetPlayerPawn _asbp_first_person_character)
  (EventDispatchers|BindEventtoOnBeginCursorOver (delegate Custom|OnCursorOver))
  (EventDispatchers|BindEventtoOnEndCursorOver (delegate Custom|OnCursorEnd)))

(event EventOnRightClick
  (params (Player :type BP%20First%20Person%20Character%20Object%20Reference))
  (CallFunction|RightClick Player))

(event EventOnLeftClick
  (params (Player :type BP%20First%20Person%20Character%20Object%20Reference))
  (CallFunction|LeftClick Player))

(fn ConstructionScript
  (Components|StaticMesh|SetStaticMesh (Variables|Default|GetStaticMesh) (Variables|Interactable|GetInteractableMesh))
  (Rendering|Material|SetMaterial (Variables|Default|GetStaticMesh) 0 (Variables|Interactable|GetInteractableMaterial)))