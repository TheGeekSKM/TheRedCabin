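; BP_REP_Wall is a wall actor that shows between zero and four board meshes to match its count.
; It stores the four board components in an ordered array on BeginPlay, then applies the current Count.
; Its OnCountUpdate override calls the parent, hides every board, then reveals that many from the start of the array.
; Counts outside that range leave board visibility unchanged.
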(event EventBeginPlay
  (|CallParentFunction)
  (Variables|Default|SetBoards (Utilities|Array|MakeArray (Variables|Default|GetSM_Boards_003) (Variables|Default|GetSM_Boards_002) (Variables|Default|GetSM_Boards_001) (Variables|Default|GetSM_Boards_004)))
  (CallFunction|OnCountUpdate (Variables|Default|GetCount)))

(event Collision|EventActorBeginOverlap
  (params (OtherActor :type Actor%20Object%20Reference))
  (|CallParentFunction OtherActor) ; This node is disabled and will not be called.\nDrag off pins to build functionality.
)

(event EventTick
  (params (DeltaSeconds :type Float%20%28single-precision%29))
  (|CallParentFunction DeltaSeconds) ; This node is disabled and will not be called.\nDrag off pins to build functionality.
)

(fn ConstructionScript
  (|CallParentFunction))

(fn OnCountUpdate
  (params (CurrentCount :type Integer))
  (|CallParentFunction CurrentCount)
  (switch int CurrentCount
    (:0
      (for _array_element (Variables|Default|GetBoards)
        (Rendering|SetVisibility _array_element false false)))
    (:1
      (for _array_element_2 (Variables|Default|GetBoards) :!label _label
        (Rendering|SetVisibility _array_element_2 false false))
      (for _index (range 0 (- CurrentCount 1))
        (Rendering|SetVisibility (Utilities|Array|Get(acopy) (Variables|Default|GetBoards) _index) true false)))
    (:2
      (goto _label))
    (:3
      (goto _label))
    (:4
      (goto _label))))