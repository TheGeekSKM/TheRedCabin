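; BP_BloodPoolOnGround is an interactable where the player uses up a required item to make a blood puddle appear on the ground.
; On BeginPlay the puddle stays visible but is hidden by teleporting it far below its origin.
; On count update it takes one required item from the player's inventory, adds a Bucket, and moves the puddle back to its relative origin.
; It then disables further interaction and calls CallFin.
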(event EventBeginPlay
  (|CallParentFunction)
  (Rendering|SetVisibility (Variables|Default|GetBloodPuddle) true false)
  (Transformation|SetRelativeLocation (Variables|Default|GetBloodPuddle) "0.000000,0.000000,-1300.000000" false true))

(event Collision|EventActorBeginOverlap
  (params (OtherActor :type Actor%20Object%20Reference))
  (|CallParentFunction OtherActor) ; This node is disabled and will not be called.\nDrag off pins to build functionality.
)

(event EventTick
  (params (DeltaSeconds :type Float%20%28single-precision%29))
  (|CallParentFunction DeltaSeconds) ; This node is disabled and will not be called.\nDrag off pins to build functionality.
)

(fn ConstructionScript
  (|CallParentFunction))

(fn OnCountUpdate
  (params (CurrentCount :type Integer))
  (bind _playerpawn (Variables|Default|GetPlayerPawn))
  (bind _ac_inventory (Variables|/Game/FirstPerson/Blueprints/BP_FirstPersonCharacter.BP_FirstPersonCharacter_C|GetAC_Inventory _playerpawn))
  (|CallParentFunction CurrentCount)
  (Default|ReduceItem _ac_inventory (Variables|Default|GetRequiredLeftClickItem) 1)
  (Default|AddItem _ac_inventory "Bucket" 1)
  (Rendering|SetVisibility (Variables|Default|GetBloodPuddle) true false)
  (CallFunction|SetInteractable false)
  (Transformation|SetRelativeLocation (Variables|Default|GetBloodPuddle) "0, 0, 0" false true)
  (Default|CallFin))