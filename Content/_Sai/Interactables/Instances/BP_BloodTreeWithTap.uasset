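; Interactable blood tree with a tap, apparently a child of a parent interactable Blueprint.
; On BeginPlay it empties its item reward list and rotates the tap's parent component once to face the player.
; Left-clicking spawns an enlarged blood puddle at the blood spawn point and destroys the tree.
; Random wood-or-blood loot logic remains in the graph but is unconnected and never runs.
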(event EventBeginPlay
  (|CallParentFunction)
  (Utilities|Array|Clear (Variables|Default|GetItemsToGive))
  (Transformation|SetWorldRotation (Variables|Default|GetParentForTap) (Math|Rotator|FindLookatRotation (Transformation|GetWorldLocation (Variables|Default|GetParentForTap)) (Transformation|GetActorLocation (Game|GetPlayerCharacter 0))) false false))

(event Collision|EventActorBeginOverlap
  (params (OtherActor :type Actor%20Object%20Reference))
  (|CallParentFunction OtherActor) ; This node is disabled and will not be called.\nDrag off pins to build functionality.
)

(event EventTick
  (params (DeltaSeconds :type Float%20%28single-precision%29))
  (|CallParentFunction DeltaSeconds) ; This node is disabled and will not be called.\nDrag off pins to build functionality.
)

(event EventLeftClick
  (params (Player :type BP%20First%20Person%20Character%20Object%20Reference) (ItemUsed :type String))
  (Game|SpawnActorfromClass "/Game/_Sai/Interactables/Instances/BP_BloodPuddle.BP_BloodPuddle_C" (Math|Transform|MakeTransform (Transformation|GetWorldLocation (Variables|Default|GetBloodSpawnPoint)) "0, 0, 0" "2.000000,2.000000,2.000000") "Undefined" "MultiplyWithRoot" 0 0)
  (Actor|DestroyActor))

(fn ConstructionScript
  (|CallParentFunction))