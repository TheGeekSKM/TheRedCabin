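; BP_BloodPuddle is an interactable blood puddle that turns a Bucket into a Bucket Of Blood.
; On LeftClick it uses the player pawn's ACInventory to consume one Bucket and add one Bucket Of Blood, then destroys itself.
; The graph makes no check that the player holds a Bucket before adding the filled one.
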(event EventBeginPlay
  (|CallParentFunction))

(event Collision|EventActorBeginOverlap
  (params (OtherActor :type Actor%20Object%20Reference))
  (|CallParentFunction OtherActor) ; This node is disabled and will not be called.\nDrag off pins to build functionality.
)

(event EventTick
  (params (DeltaSeconds :type Float%20%28single-precision%29))
  (|CallParentFunction DeltaSeconds) ; This node is disabled and will not be called.\nDrag off pins to build functionality.
)

(event EventLeftClick
  (params (Player :type BP%20First%20Person%20Character%20Object%20Reference) (ItemUsed :type String))
  (bind _playerpawn (Variables|Default|GetPlayerPawn))
  (bind _ac_inventory (Variables|/Game/FirstPerson/Blueprints/BP_FirstPersonCharacter.BP_FirstPersonCharacter_C|GetAC_Inventory _playerpawn))
  (Default|ReduceItem _ac_inventory "Bucket" 1)
  (Default|AddItem _ac_inventory "Bucket Of Blood" 1)
  (Actor|DestroyActor))

(fn ConstructionScript
  (|CallParentFunction))