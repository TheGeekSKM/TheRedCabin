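; BP_Tree is an interactable tree instance that prepares randomized Wood and Blood item lists.
; On BeginPlay it fills ItemsToGive with Wood and ItemsToGiveBlod with Blood, each a random number of times.
; It also rolls against ChanceOfBeingBloodTree, but the result does nothing.
; Nodes to spawn a scaled-down BP_BloodTreeNoTap and destroy this actor are disconnected and never run.
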(event EventBeginPlay
  (|CallParentFunction)
  (Utilities|FlowControl|Sequence
    (:then_0
      (for _index (range 0 (Math|Random|RandomIntegerinRange 2 9))
        (Utilities|Array|Add (Variables|Default|GetItemsToGive) "Wood")))
    (:then_1
      (for _index_2 (range 0 (Math|Random|RandomIntegerinRange 2 9))
        (Utilities|Array|Add (Variables|Default|GetItemsToGiveBlod) "Blood")))
    (:then_2
      (if (<= (Math|Random|RandomFloatinRange 1.0 1e+02) (Variables|Default|GetChanceOfBeingBloodTree))
        _))))

(event Collision|EventActorBeginOverlap
  (params (OtherActor :type Actor%20Object%20Reference))
  (|CallParentFunction OtherActor) ; This node is disabled and will not be called.\nDrag off pins to build functionality.
)

(event EventTick
  (params (DeltaSeconds :type Float%20%28single-precision%29))
  (|CallParentFunction DeltaSeconds) ; This node is disabled and will not be called.\nDrag off pins to build functionality.
)

(fn ConstructionScript
  (|CallParentFunction))