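; BP_BloodTreeNoTap is the untapped "Bleeding Tree" interactable, which the player converts into a tapped tree.
; BeginPlay sets the inherited name, left-click hint and required item, a Tap needed to drain it.
; LeftClick swaps the actor by spawning BP_BloodTreeWithTap at the same location and rotation with a fixed reduced scale, then destroying itself.
; The graph itself has no item check.
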(event EventBeginPlay
  (|CallParentFunction)
  (Variables|Default|SetRequiredLeftClickItem "Tap")
  (Variables|Default|SetLeftClickInfo "Needs Tap to Drain")
  (Variables|Default|SetInteractableName "Bleeding Tree"))

(event Collision|EventActorBeginOverlap
  (params (OtherActor :type Actor%20Object%20Reference))
  (|CallParentFunction OtherActor) ; This node is disabled and will not be called.\nDrag off pins to build functionality.
)

(event EventTick
  (params (DeltaSeconds :type Float%20%28single-precision%29))
  (|CallParentFunction DeltaSeconds) ; This node is disabled and will not be called.\nDrag off pins to build functionality.
)

(event EventLeftClick
  (params (Player :type BP%20First%20Person%20Character%20Object%20Reference) (ItemUsed :type String))
  (bind _returnvalue (Transformation|GetActorTransform))
  (Game|SpawnActorfromClass "/Game/_Sai/Interactables/Instances/BP_BloodTreeWithTap.BP_BloodTreeWithTap_C" (Math|Transform|MakeTransform (.location _returnvalue) (.rotation _returnvalue) "0.300000,0.300000,0.300000") "Undefined" "MultiplyWithRoot" 0 0)
  (Actor|DestroyActor))

(fn ConstructionScript
  (|CallParentFunction))