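; Base class for first-person interactables, with overridable left and right click actions and an optional construction-time mesh, material and transform setup.
; Hovering shows name and click prompts in the player's interaction widget and toggles the mesh's custom depth stencil.
; Each click is gated by enable flags and an optional inventory item, which may need equipping in the matching hand.
; Item checks rerun each tick while hovered, and successful clicks call success hooks.
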(event Custom|SetInteractable
  (params (CanInteract :type Boolean))
  (bind _output_get (Variables|Default|SetCanInteract CanInteract))
  (if (not _output_get)
    (CallFunction|OnExitHover)))

(event Custom|LeftClick
  (params (Player :type BP%20First%20Person%20Character%20Object%20Reference) (ItemUsed :type String)))

(event Custom|RightClick
  (params (Player :type BP%20First%20Person%20Character%20Object%20Reference) (ItemUsed :type String)))

(event EventBeginPlay
  (bind _asbp_first_person_character (Utilities|Casting|CastToBP_FirstPersonCharacter (Game|GetPlayerCharacter 0)))
  (Variables|Default|SetPlayerPawn _asbp_first_person_character)
  (Variables|Interactable|SetBaseStencil (Variables|/Script/Engine.PrimitiveComponent|GetCustomDepthStencilValue (Variables|Default|GetStaticMesh)))
  (Rendering|SetCustomDepthStencilValue (Variables|Default|GetStaticMesh) 0))

(event EventTick
  (params (DeltaSeconds :type Float%20%28single-precision%29))
  (if (Variables|Default|GetIsHovering)
    (CallFunction|CheckLeftItem)
    (CallFunction|CheckRightItem)))

(event EventOnHover
  (if (Variables|Default|GetCanInteract)
    (Variables|Default|SetIsHovering true)
    (CallFunction|CheckLeftItem)
    (CallFunction|CheckRightItem)
    (Default|ShowHover (Variables|/Game/FirstPerson/Blueprints/BP_FirstPersonCharacter.BP_FirstPersonCharacter_C|GetInteractionWidget (Variables|Default|GetPlayerPawn)) (Variables|Interactable|GetInteractableName) (CallFunction|GetLeftInfo) (CallFunction|GetRightInfo))
    (Rendering|SetCustomDepthStencilValue (Variables|Default|GetStaticMesh) (Variables|Interactable|GetBaseStencil))))

(event EventOnRightClick
  (params (Player :type BP%20First%20Person%20Character%20Object%20Reference) (ItemUsed :type String))
  (if (Variables|Default|GetCanInteract)
    (bind _itemnotrequired (CallFunction|CheckRightItem))
    (if _itemnotrequired
      (CallFunction|RightClick Player ItemUsed)
      (Default|CallOnSuccessfulRight :!label _label)
      (elif (Variables|ItemUsage|GetRightClickItemFound)
        (CallFunction|RightClick Player ItemUsed)
        (goto _label)))))

(event EventOnLeftClick
  (params (Player :type BP%20First%20Person%20Character%20Object%20Reference) (ItemUsed :type String))
  (if (Variables|Default|GetCanInteract)
    (bind _itemnotrequired (CallFunction|CheckLeftItem))
    (if _itemnotrequired
      (CallFunction|LeftClick Player ItemUsed)
      (Default|CallOnSuccessfulLeft :!label _label)
      (elif (Variables|ItemUsage|GetLeftClickItemFound)
        (CallFunction|LeftClick Player ItemUsed)
        (goto _label)))))

(event EventOnExitHover
  (bind _playerpawn (Variables|Default|GetPlayerPawn))
  (bind _interactionwidget (Variables|/Game/FirstPerson/Blueprints/BP_FirstPersonCharacter.BP_FirstPersonCharacter_C|GetInteractionWidget _playerpawn))
  (Utilities|IsValid _interactionwidget
    (:Is%20Valid
      (Default|HideHover _interactionwidget)
      (Variables|Default|SetIsHovering false)
      (Rendering|SetCustomDepthStencilValue (Variables|Default|GetStaticMesh) 0))))

(event EventDestroyed
  (CallFunction|OnExitHover))

(fn ConstructionScript
  (if (Variables|Default|GetUseMeshMatVariables)
    (Components|StaticMesh|SetStaticMesh (Variables|Default|GetStaticMesh) (Variables|Interactable|GetInteractableMesh))
    (Rendering|Material|SetMaterial (Variables|Default|GetStaticMesh) 0 (Variables|Interactable|GetInteractableMaterial))
    (Transformation|SetRelativeTransform (Variables|Default|GetStaticMesh) (Variables|Interactable|GetMesh%20Transform) false false)))

(fn GetRightInfo
  (if (Variables|ItemUsage|GetRightClickItemFound)
    (return (Variables|ItemUsage|GetRightClickInfoItem))
    (else
      (return (Variables|Interactable|GetRightClickInfo)))))

(fn GetLeftInfo
  (if (Variables|ItemUsage|GetLeftClickItemFound)
    (return (Variables|ItemUsage|GetLeftClickInfoItem))
    (else
      (return (Variables|Interactable|GetLeftClickInfo)))))

(fn CheckLeftItem
  ;[0.15 0.15 0.15 0.5] Can we Interact
  (if (Variables|Default|GetCanLeftInteract)
    ;[0.15 0.15 0.15 0.5] Do we require an item
    (if (not (Utilities|Enum|Equal(Enum) (Variables|ItemUsage|GetRequiredLeftClickItem) ""))
      ;[0.15 0.15 0.15 0.5] Does the Player Exist
      (Utilities|IsValid (Variables|Default|GetPlayerPawn)
        (:Is%20Valid
          ;[0.15 0.15 0.15 0.5] Is the Left Click Item in the Player's Inventory
          (if (> (Default|GetItemCount (Variables|/Game/FirstPerson/Blueprints/BP_FirstPersonCharacter.BP_FirstPersonCharacter_C|GetAC_Inventory (Variables|Default|GetPlayerPawn)) (Variables|ItemUsage|GetRequiredLeftClickItem)) 0)
            (if (not (Variables|ItemUsage|GetRequiresEquipped))
              (Variables|ItemUsage|SetLeftClickItemFound true :!label _label)
              (else
                ;[0.15 0.15 0.15 0.5] Is the Required Item Currently Equipped
                (if (Utilities|Enum|Equal(Enum) (Variables|/Game/_Sai/Inventory/AC_Inventory.AC_Inventory_C|GetLeftHandItem (Variables|/Game/FirstPerson/Blueprints/BP_FirstPersonCharacter.BP_FirstPersonCharacter_C|GetAC_Inventory (Variables|Default|GetPlayerPawn))) (Variables|ItemUsage|GetRequiredLeftClickItem))
                  (goto _label)
                  (else
                    (Variables|ItemUsage|SetLeftClickItemFound false)))))
            (else
              (Variables|ItemUsage|SetLeftClickItemFound false))))
        (:Is%20Not%20Valid
          (Variables|ItemUsage|SetLeftClickItemFound false)))
      (return false)
      (else
        (return true)))
    (else
      (return false))))

(fn CheckRightItem
  ;[0.15 0.15 0.15 0.5] Can we Interact
  (if (Variables|Default|GetCanRightInteract)
    ;[0.15 0.15 0.15 0.5] Do we require an item
    (if (not (Utilities|Enum|Equal(Enum) (Variables|ItemUsage|GetRequiredRightClickItem) ""))
      ;[0.15 0.15 0.15 0.5] Does the Player Exist
      (Utilities|IsValid (Variables|Default|GetPlayerPawn)
        (:Is%20Valid
          ;[0.15 0.15 0.15 0.5] Is the Left Click Item in the Player's Inventory
          (if (> (Default|GetItemCount (Variables|/Game/FirstPerson/Blueprints/BP_FirstPersonCharacter.BP_FirstPersonCharacter_C|GetAC_Inventory (Variables|Default|GetPlayerPawn)) (Variables|ItemUsage|GetRequiredRightClickItem)) 0)
            (if (not (Variables|ItemUsage|GetRequiresEquipped))
              (Variables|ItemUsage|SetRightClickItemFound true :!label _label)
              (else
                ;[0.15 0.15 0.15 0.5] Is the Required Item Currently Equipped
                (if (Utilities|Enum|Equal(Enum) (Variables|/Game/_Sai/Inventory/AC_Inventory.AC_Inventory_C|GetRightHandItem (Variables|/Game/FirstPerson/Blueprints/BP_FirstPersonCharacter.BP_FirstPersonCharacter_C|GetAC_Inventory (Variables|Default|GetPlayerPawn))) (Variables|ItemUsage|GetRequiredRightClickItem))
                  (goto _label)
                  (else
                    (Variables|ItemUsage|SetRightClickItemFound false)))))
            (else
              (Variables|ItemUsage|SetRightClickItemFound false))))
        (:Is%20Not%20Valid
          (Variables|ItemUsage|SetRightClickItemFound false)))
      (return false)
      (else
        (return true)))
    (else
      (return false))))