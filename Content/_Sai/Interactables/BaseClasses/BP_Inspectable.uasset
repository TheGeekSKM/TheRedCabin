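; BP_Inspectable is an interactable base class for objects the player can inspect by left-clicking.
; A left click passes itself to the player as the inspect item, hides its static mesh and ends the hover state.
; PlaceBack either adds a configured item and count to the given inventory and destroys the actor, or makes the mesh visible again, depending on DoesGiveItem.
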(event Custom|PlaceBack
  (params (Inventory :type AC%20Inventory%20Object%20Reference))
  (if (Variables|Inspectable|GetDoesGiveItem)
    (Default|AddItem Inventory (Variables|Inspectable|GetItemToGivePlayer) (Variables|Inspectable|GetNumItemsToGive))
    (Actor|DestroyActor)
    (else
      (Rendering|SetVisibility (Variables|Default|GetStaticMesh) true false))))

(event EventBeginPlay
  (|CallParentFunction) ; This node is disabled and will not be called.\nDrag off pins to build functionality.
)

(event Collision|EventActorBeginOverlap
  (params (OtherActor :type Actor%20Object%20Reference)))

(event EventTick
  (params (DeltaSeconds :type Float%20%28single-precision%29)))

(event EventOnLeftClick
  (params (Player :type BP%20First%20Person%20Character%20Object%20Reference) (ItemUsed :type String))
  (Default|SetInspectItem Player self)
  (Rendering|SetVisibility (Variables|Default|GetStaticMesh) false false)
  (CallFunction|OnExitHover))

(fn ConstructionScript
  (|CallParentFunction))