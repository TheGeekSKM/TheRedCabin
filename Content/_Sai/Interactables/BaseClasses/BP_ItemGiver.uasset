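; BP_ItemGiver is an interactable that gives the player an item when left-clicked.
; OnLeftClick checks that CurrentIndex is within ItemsToGive, then adds one of that named item to the player's ACInventory component.
; The graph never advances CurrentIndex, so repeated clicks give the same entry unless the index changes elsewhere.
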(event EventBeginPlay
  (|CallParentFunction) ; This node is disabled and will not be called.\nDrag off pins to build functionality.
)

(event Collision|EventActorBeginOverlap
  (params (OtherActor :type Actor%20Object%20Reference)))

(event EventTick
  (params (DeltaSeconds :type Float%20%28single-precision%29))
  (|CallParentFunction DeltaSeconds) ; This node is disabled and will not be called.\nDrag off pins to build functionality.
)

(event EventOnLeftClick
  (params (Player :type BP%20First%20Person%20Character%20Object%20Reference) (ItemUsed :type String))
  (if (< (Variables|Default|GetCurrentIndex) (Utilities|Array|Length (Variables|Default|GetItemsToGive)))
    (Default|AddItem (Variables|/Game/FirstPerson/Blueprints/BP_FirstPersonCharacter.BP_FirstPersonCharacter_C|GetAC_Inventory Player) (Utilities|Array|Get(acopy) (Variables|Default|GetItemsToGive) (Variables|Default|GetCurrentIndex)) 1)))

(fn ConstructionScript
  (|CallParentFunction))