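; Base trigger-box interactable that signals when the first-person character enters, exits or faces a given direction inside it.
; Box overlaps track the pawn and fire enter and exit calls, optionally destroying the actor afterwards.
; With CheckRotation on, those calls are skipped and Tick compares player and actor forward vectors by dot product, firing a facing call on a five-second cooldown.
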(event OnComponentBeginOverlap(Box)
  (params (OverlappedComponent :type Primitive%20Component%20Object%20Reference) (OtherActor :type Actor%20Object%20Reference) (OtherComp :type Primitive%20Component%20Object%20Reference) (OtherBodyIndex :type Integer) (bFromSweep :type Boolean) (SweepResult :type Hit%20Result%20Structure%20%28by%20ref%29))
  (bind _asbp_first_person_character (Utilities|Casting|CastToBP_FirstPersonCharacter OtherActor))
  (Variables|Default|SetPawn _asbp_first_person_character)
  (Variables|Default|SetPlayerIn true)
  (if (not (Variables|Default|GetCheckRotation))
    (Default|CallPlayerEnter _asbp_first_person_character)
    (Utilities|DoOnceLogic)))

(event OnComponentEndOverlap(Box)
  (params (OverlappedComponent :type Primitive%20Component%20Object%20Reference) (OtherActor :type Actor%20Object%20Reference) (OtherComp :type Primitive%20Component%20Object%20Reference) (OtherBodyIndex :type Integer))
  (bind _asbp_first_person_character (Utilities|Casting|CastToBP_FirstPersonCharacter OtherActor))
  (Variables|Default|SetPawn 0)
  (Variables|Default|SetPlayerIn false)
  (if (not (Variables|Default|GetCheckRotation))
    (Default|CallPlayerExit _asbp_first_person_character)
    (Utilities|DoOnceLogic)))

(event EventBeginPlay)

(event Collision|EventActorBeginOverlap
  (params (OtherActor :type Actor%20Object%20Reference)))

(event EventTick
  (params (DeltaSeconds :type Float%20%28single-precision%29))
  (if (and (Variables|Default|GetPlayerIn) (Variables|Default|GetCheckRotation))
    (Utilities|IsPlayerFacingMyDirection
      (:true
        (Utilities|FlowControl|DoOnce false :!label _label
          (:Completed
            (Default|CallPlayerFacingDirection (Variables|Default|GetPawn))
            (Utilities|FlowControl|Delay 5.0)
            (goto _label Reset)))))))

(fn ConstructionScript)