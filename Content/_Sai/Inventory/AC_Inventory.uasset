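; Inventory actor component that stores item counts in a name-keyed map and tracks items equipped to left-click and right-click hand slots.
; Events add, reduce, equip and unequip items; reducing subtracts without clamping or removing entries.
; EquipNext and EquipPrevious cycle the left-hand item through the map's key order with wraparound, including zero-count entries.
; A Debug-gated log prints items with positive counts and marks equipped ones.
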(event Custom|EquipFirstItem
  (bind _inventory (Variables|Default|GetInventory))
  (if (> (Utilities|Map|Length _inventory) 0)
    (Variables|Default|SetLeftHandItem (.Key (Utilities|Map|GetKeyValueByIndex _inventory 0)))))

(event Custom|AddItem
  (params (Name :type String) (Count :type Integer))
  (bind _inventory (Variables|Default|GetInventory))
  (if (Utilities|Map|Contains (Variables|Default|GetInventory) Name)
    (Utilities|Map|Add _inventory Name (+ (.Value (Utilities|Map|Find _inventory Name)) Count))
    (else
      (Utilities|Map|Add (Variables|Default|GetInventory) Name Count))))

(event Custom|LogInventory
  (if (Variables|Default|GetDebug)
    (bind (_keypin _valuepin) (Utilities|Map|ForEachLoop(Map) (Variables|Default|GetInventory))
      (:then
        (if (> (CallFunction|GetItemCount _keypin) 0)
          (if (.Equipped (CallFunction|CheckifEquipped _keypin))
            (Development|PrintText (Utilities|Text|FormatText "- [Equipped] \"{name}\" x{count}" _keypin _valuepin) true true "(R=1.000000,G=0.481274,B=0.078720,A=1.000000)" 5.0)
            (else
              (Development|PrintText (Utilities|Text|FormatText "- \"{name}\" x{count}" _keypin _valuepin) true true "(R=1.000000,G=0.481274,B=0.078720,A=1.000000)" 5.0)))))
      (:CompletedPin
        (Development|PrintText "INVENTORY:" true true "(R=1.000000,G=0.481274,B=0.078720,A=1.000000)" 5.0)))))

(event Custom|ReduceItem
  (params (ItemName :type String) (UsageAmount :type Integer))
  (bind _inventory (Variables|Default|GetInventory))
  (bind (_value _returnvalue) (Utilities|Map|Find _inventory ItemName))
  (if _returnvalue
    (Utilities|Map|Add _inventory ItemName (- _value UsageAmount))))

(event Custom|EquipItem
  (params (Right :type Boolean) (ItemName :type String))
  (if (Utilities|Map|Contains (Variables|Default|GetInventory) ItemName)
    (if Right
      (bind _output_get (Variables|Default|SetRightHandItem ItemName))
      (Development|PrintText (Utilities|Text|FormatText "[INVENTORY] Equipped {itemName} to Right Click" _output_get))
      (else
        (bind _output_get_2 (Variables|Default|SetLeftHandItem ItemName))
        (Development|PrintText (Utilities|Text|FormatText "[INVENTORY] Equipped {itemName} to Left Click" _output_get_2))))))

(event Custom|UnequipSlot
  (params (Right :type Boolean))
  (if Right
    (Variables|Default|SetRightHandItem "")
    (else
      (Variables|Default|SetLeftHandItem ""))))

(fn CheckifEquipped
  (params (ItemName :type String))
  (if (Utilities|Enum|Equal(Enum) ItemName (Variables|Default|GetLeftHandItem))
    (return true "NewEnumerator2")
    (elif (Utilities|Enum|Equal(Enum) ItemName (Variables|Default|GetRightHandItem))
      (return true "NewEnumerator1")
      (else
        (return false "NewEnumerator0")))))

(fn GetItemCount
  (params (ItemName :type String))
  (return (.Value (Utilities|Map|Find (Variables|Default|GetInventory) ItemName))))

(fn EquipNext
  (if (Utilities|Map|Contains (Variables|Default|GetInventory) (Variables|Default|GetLeftHandItem))
    ;[0.15 0.15 0.15 0.5] Get Current Index for Equipped Item
    (bind _keys (Utilities|Map|Keys (Variables|Default|GetInventory)))
    (bind (_array_element _array_index) (Utilities|Array|ForEachLoopwithBreak _keys :!label _label)
      (:LoopBody
        (if (Utilities|Enum|Equal(Enum) _array_element (Variables|Default|GetLeftHandItem))
          (LocalVariables|SetCurrentItemIndex _array_index)
          (goto _label Break)))
      (:Completed
        ;[0.15 0.15 0.15 0.5] If currentIndex++ > inventoryLength
        (bind _keys_2 (Utilities|Map|Keys (Variables|Default|GetInventory)))
        (if (>= (+ (LocalVariables|GetCurrentItemIndex) 1) (Utilities|Array|Length _keys_2))
          (bind _output_get (LocalVariables|SetCurrentItemIndex 0))
          (else
            ;[0.15 0.15 0.15 0.5] increment current item index
            (bind _result (Math|Integer|IncrementInt (LocalVariables|GetCurrentItemIndex))
              (:%20%20
                (bind _keys_3 (Utilities|Map|Keys (Variables|Default|GetInventory)))
                (LocalVariables|SetCurrentItemIndex (Math|Integer|Clamp(Integer) _result 0 (Utilities|Array|Length _keys_3)))))))
        (CallFunction|EquipItem false (.Key (Utilities|Map|GetKeyValueByIndex (Variables|Default|GetInventory) _output_get)))))))

(fn EquipPrevious
  (if (Utilities|Map|Contains (Variables|Default|GetInventory) (Variables|Default|GetLeftHandItem))
    ;[0.15 0.15 0.15 0.5] Get Current Index for Equipped Item
    (bind _keys (Utilities|Map|Keys (Variables|Default|GetInventory)))
    (bind (_array_element _array_index) (Utilities|Array|ForEachLoopwithBreak _keys :!label _label)
      (:LoopBody
        (if (Utilities|Enum|Equal(Enum) _array_element (Variables|Default|GetLeftHandItem))
          (LocalVariables|SetCurrentItemIndex _array_index)
          (goto _label Break)))
      (:Completed
        ;[0.15 0.15 0.15 0.5] If currentIndex-- < 0
        (if (< (- (LocalVariables|GetCurrentItemIndex) 1) 0)
          ;[0.15 0.15 0.15 0.5] Get Item at Last Index
          (bind _keys_2 (Utilities|Map|Keys (Variables|Default|GetInventory)))
          (bind _output_get (LocalVariables|SetCurrentItemIndex (Utilities|Array|LastIndex _keys_2)))
          (else
            ;[0.15 0.15 0.15 0.5] decrement current item index
            (bind _result (Math|Integer|DecrementInt (LocalVariables|GetCurrentItemIndex))
              (:%20%20
                (bind _keys_3 (Utilities|Map|Keys (Variables|Default|GetInventory)))
                (LocalVariables|SetCurrentItemIndex (Math|Integer|Clamp(Integer) _result 0 (Utilities|Array|Length _keys_3)))))))
        (CallFunction|EquipItem false (.Key (Utilities|Map|GetKeyValueByIndex (Variables|Default|GetInventory) _output_get)))))))