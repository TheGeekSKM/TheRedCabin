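; BP_Repairable_Base is a base Blueprint, named for repairable objects, that tracks a click-driven counter.
; LeftClick increments Count and RightClick decrements it, with both paths clamping the value between zero and CountLimit.
; Each click then passes the new value to OnCountUpdate, an empty function here that serves as a hook for reacting to the change.
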(event EventBeginPlay
  (|CallParentFunction) ; This node is disabled and will not be called.\nDrag off pins to build functionality.
)

(event Collision|EventActorBeginOverlap
  (params (OtherActor :type Actor%20Object%20Reference)))

(event EventTick
  (params (DeltaSeconds :type Float%20%28single-precision%29)))

(event EventLeftClick
  (params (Player :type BP%20First%20Person%20Character%20Object%20Reference))
  (Math|Integer|IncrementInt (Variables|Default|GetCount)
    (:%20%20
      (bind _output_get (Variables|Default|SetCount (Math|Integer|Clamp(Integer) (Variables|Default|GetCount) 0 (Variables|Default|GetCountLimit))))
      (CallFunction|OnCountUpdate _output_get))))

(event EventRightClick
  (params (Player :type BP%20First%20Person%20Character%20Object%20Reference))
  (Math|Integer|DecrementInt (Variables|Default|GetCount)
    (:%20%20
      (bind _output_get (Variables|Default|SetCount (Math|Integer|Clamp(Integer) (Variables|Default|GetCount) 0 (Variables|Default|GetCountLimit))))
      (CallFunction|OnCountUpdate _output_get))))

(fn ConstructionScript
  (|CallParentFunction))

(fn OnCountUpdate
  (params (CurrentCount :type Integer)))